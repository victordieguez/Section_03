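; Player-controllable tank Blueprint that routes input to track throttles, aim rotation and firing.
; On BeginPlay it hands its Turret, Barrel and both track components to setter functions defined outside these graphs.
; Separate left and right throttle axes drive each track independently.
; Aim axes yaw an azimuth gimbal and pitch the spring arm without moving turret or barrel directly, and the Fire action calls Fire.
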(event `self.ReceiveBeginPlay`
  (`self.SetTurret` (`self.Turret`))
  (`self.SetBarrel` (`self.Barrel`))
  (`self.SetRightTrack` (`self.Right Track`))
  (`self.SetLeftTrack` (`self.Left Track`)))

(event `InputAxis|AimElevation`
  (params (AxisValue :type "Float (single-precision)"))
  (`SceneComponent.K2_AddLocalRotation` (`self.SpringArm`) (`KismetMathLibrary.MakeRotator` 0.0 AxisValue) false false))

(event `InputAxis|Left Track Throttle`
  (params (AxisValue :type "Float (single-precision)"))
  (`TankTrack.SetThrottle` (`self.Left Track`) AxisValue))

(event `InputAxis|AimAzimuth`
  (params (AxisValue :type "Float (single-precision)"))
  (`SceneComponent.K2_AddLocalRotation` (`self.AzimuthGimbal`) (`KismetMathLibrary.MakeRotator` 0.0 0.0 AxisValue) false false))

(event `InputAxis|Right Track Throttle`
  (params (AxisValue :type "Float (single-precision)"))
  (`TankTrack.SetThrottle` (`self.Right Track`) AxisValue))

(event `InputAction|Fire`
  (params (Key :type "Key Structure"))
  (:`Pressed`
    (`self.Fire`)))

(fn `UserConstructionScript`)